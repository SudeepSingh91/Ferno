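; Player character that moves freely until it possesses a nearby PossessPoint actor, and is sent back to its start transform when its decay timer runs out.
; Tick sphere-searches for points while free; possessing hides the cube, lerps onto the point and then follows it.
; Releasing hops to another point in range or lerps to the Release component's position and resets the timer.
; A small upward impulse applies while falling.
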(event Custom|PossessInRange
  (bind _outactors (Class|KismetSystemLibrary|SphereOverlapActorsNEW (Transformation|GetActorLocation) 1.8e+02 (Utilities|Array|MakeArray "ObjectTypeQuery2") "/Game/Blueprints/PossessPoint.PossessPoint_C"))
  (if (== (Utilities|Array|Length _outactors) 0)
    (Variables|Default|SetPossPoint (Variables|Default|GetNullPoint))
    (else
      (for _array_element _outactors
        (Variables|Default|SetPossPoint (Transformation|GetActorTransform _array_element))
        (bind _aspossess_point (Utilities|Casting|CastToPossessPoint _array_element))
        (Variables|Default|SetPoint _aspossess_point)))))

(event Custom|AttemptToPossess
  (if (not (== (Variables|Default|GetPossPoint) (Variables|Default|GetNullPoint)))
    (Variables|Default|SetIsPossess true)))

(event EventBeginPlay
  (Variables|Default|SetRespawnPos (Transformation|GetActorTransform)))

(event EventTick
  (params (DeltaSeconds :type Float%20%28single-precision%29))
  (Variables|Default|SetDeltaTime DeltaSeconds)
  (if (AI|Components|NavMovement|IsFalling (Variables|Character|GetCharacterMovement))
    (Physics|AddImpulse (Variables|Character|GetCharacterMovement) (Math|Vector|MakeVector 0.0 0.0 1.0) false))
  (if (Variables|Default|GetIsPossess)
    (if (Variables|Default|GetInProcess)
      (CallFunction|UnPossessPoint)
      (else
        (CallFunction|PossessPoint)))
    (else
      (CallFunction|PossessinRange)
      (bind _output_get (Variables|Default|SetDecayTimer (- (Variables|Default|GetDecayTimer) DeltaSeconds)))
      (if (<= _output_get 0.0)
        (CallFunction|Respawn DeltaSeconds)))))

(event Input|ActionEvents|InputActionPossessPoint
  (params (Key :type Key%20Structure :default "AnyKey"))
  (:Pressed
    (if (Variables|Default|GetIsPossess)
      (Variables|Default|SetReleasePoint (Transformation|GetWorldTransform (Variables|Default|GetRelease)))
      (Variables|Default|SetInProcess true)
      (Variables|Default|SetTransitionAmount 0.0)
      (else
        (CallFunction|AttempttoPossess)))))

(event Input|AxisEvents|InputAxisForward
  (params (AxisValue :type Float%20%28single-precision%29))
  (if (not (Variables|Default|GetIsPossess))
    (Pawn|Input|AddMovementInput (Transformation|GetActorForwardVector) AxisValue false)))

(event Input|AxisEvents|InputAxisSideway
  (params (AxisValue :type Float%20%28single-precision%29))
  (if (not (Variables|Default|GetIsPossess))
    (Pawn|Input|AddMovementInput (Transformation|GetActorRightVector) AxisValue false)))

(fn ConstructionScript)

(fn Respawn
  (params (Delta :type Float%20%28single-precision%29))
  (Rendering|SetVisibility (Variables|Default|GetCube) false false)
  (bind _output_get (Variables|Default|SetTransitionAmount (Math|Float|Clamp(Float) (+ (* Delta 2.0) (Variables|Default|GetTransitionAmount)))))
  (Transformation|SetActorTransform (Math|Transform|Lerp(Transform) (Transformation|GetActorTransform) (Variables|Default|GetRespawnPos) _output_get))
  (if (>= (Variables|Default|GetTransitionAmount) 1.0)
    (Rendering|SetVisibility (Variables|Default|GetCube) true false)
    (Variables|Default|SetTransitionAmount 0.0)
    (Variables|Default|SetDecayTimer 3.0)))

(fn PossessPoint
  (if (<= (Variables|Default|GetTransitionAmount) 0.5)
    (Rendering|SetVisibility (Variables|Default|GetCube) false false)
    (bind _output_get (Variables|Default|SetTransitionAmount (Math|Float|Clamp(Float) (+ (* (Variables|Default|GetDeltaTime) 2.0) (Variables|Default|GetTransitionAmount)))))
    (Transformation|SetActorTransform (Math|Transform|Lerp(Transform) (Transformation|GetActorTransform) (Variables|Default|GetPossPoint) _output_get))
    (else
      (Transformation|SetActorTransform (Transformation|GetActorTransform (Variables|Default|GetPoint))))))

(fn UnPossessPoint
  (bind _outactors (Class|KismetSystemLibrary|SphereOverlapActorsNEW (Transformation|GetActorLocation) 1.8e+02 (Utilities|Array|MakeArray "ObjectTypeQuery2") "/Game/Blueprints/PossessPoint.PossessPoint_C" (Utilities|Array|MakeArray (Variables|Default|GetPoint))))
  (if (== (Utilities|Array|Length _outactors) 0)
    (bind _output_get (Variables|Default|SetTransitionAmount (Math|Float|Clamp(Float) (+ (* (Variables|Default|GetDeltaTime) 3.0) (Variables|Default|GetTransitionAmount)))))
    (Transformation|SetActorTransform (Math|Transform|Lerp(Transform) (Transformation|GetActorTransform) (Variables|Default|GetReleasePoint) _output_get))
    (if (>= (Variables|Default|GetTransitionAmount) 1.0)
      (Variables|Default|SetTransitionAmount 0.0)
      (Variables|Default|SetInProcess false)
      (Variables|Default|SetIsPossess false)
      (Variables|Default|SetDecayTimer 3.0)
      (Rendering|SetVisibility (Variables|Default|GetCube) true false)
      (Transformation|SetActorRotation "0,90.000000, 0"))
    (else
      (bind _array_element (Utilities|Array|ForEachLoopwithBreak _outactors)
        (:LoopBody
          (Variables|Default|SetPossPoint (Transformation|GetActorTransform _array_element))
          (bind _aspossess_point (Utilities|Casting|CastToPossessPoint _array_element))
          (Variables|Default|SetPoint _aspossess_point)
          (Variables|Default|SetInProcess false)
          (CallFunction|PossessPoint))))))